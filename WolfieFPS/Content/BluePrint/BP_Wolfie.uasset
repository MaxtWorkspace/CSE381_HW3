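; BP_Wolfie is an AI-controlled pawn that wanders randomly and fires the ball it holds.
; Tick calls Fire whenever BallInHand is valid, then paces movement with a randomized Delay before AIMoveTo heads to a nearby reachable point.
; IsMoving is set during each move and cleared on success or failure.
; When IsBoss is set, destinations are flattened onto a fixed X line, keeping only random Y and Z.
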(event `self.ReceiveTick`
  (params (DeltaSeconds :type "Float (single-precision)"))
  (bind _randomlocation (`NavigationSystemV1.K2_GetRandomReachablePointInRadius` (`self.K2_GetActorLocation`) 1000.0 null null))
  (if (`KismetSystemLibrary.IsValid` (`self.ballInHand`))
    (`self.Fire`))
  (`KismetSystemLibrary.Delay` (`KismetMathLibrary.RandomFloatInRange` 0.5 3.0))
  (set `self.IsMoving` true)
  (if (`self.IsBoss`)
    (`|AIMoveTo` self (+ (* _randomlocation (0.0 1.0 1.0)) (-1168.0 0.0 0.0)) null
      (:`OnSuccess`
        _)
      (:`OnFail`
        _))
    (else
      (`|AIMoveTo` self _randomlocation null
        (:`OnSuccess`
          _)
        (:`OnFail`
          _))))
  (set `self.IsMoving` false))

(fn `UserConstructionScript`)